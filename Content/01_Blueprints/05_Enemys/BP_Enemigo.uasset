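; Enemy Blueprint that tracks a health value and destroys itself when that health runs out.
; Each Daño (damage) event subtracts a fixed amount from Vida (health) and prints the new value to the screen.
; At zero or below the actor is destroyed; otherwise the value is printed again, and the construction script is empty.
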(event EventDaño
  (params (Dano :type Float%20%28double-precision%29))
  (bind _output_get (Variables|Default|SetVida (- (Variables|Default|GetVida) 0.5)))
  (Development|PrintString (Utilities|String|ToString(Float) (Variables|Default|GetVida)))
  (if (<= _output_get 0.0)
    (Actor|DestroyActor)
    (else
      (Development|PrintString (Utilities|String|ToString(Float) (Variables|Default|GetVida))))))

(fn ConstructionScript)