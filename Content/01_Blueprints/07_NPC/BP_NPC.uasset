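; BP_NPC is an interactable NPC that shows its dialogue one line at a time on screen.
; Each Interact call writes the next Dialogos entry into a WB_Dialogo widget, which is created for player controller 0 when no valid one exists.
; An Interact call after the last line removes the widget, clears its reference and resets DialogueIndex, so the conversation can replay.
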(event EventInteract
  (if (< (Variables|Default|GetDialogueIndex) (Utilities|Array|Length (Variables|Default|GetDialogos)))
    (Variables|Default|GetDialogueRef
      (:then
        _)
      (:else
        (bind _returnvalue (UserInterface|CreateWidget "/Game/01_Blueprints/06_Widget/WB_Dialogo.WB_Dialogo_C" (Game|GetPlayerController 0)))
        (bind _output_get (Variables|Default|SetDialogueRef _returnvalue))
        (UserInterface|Viewport|AddtoViewport _output_get 0)))
    (Rendering|Components|TextRender|SetText (Variables|/Game/01_Blueprints/06_Widget/WB_Dialogo.WB_Dialogo_C|GetDialoge (Variables|Default|GetDialogueRef)) (Utilities|Text|ToText(String) (Utilities|Array|Get(acopy) (Variables|Default|GetDialogos) (Variables|Default|GetDialogueIndex))))
    (Math|Integer|IncrementInt (Variables|Default|GetDialogueIndex))
    (else
      (Widget|RemovefromParent (Variables|Default|GetDialogueRef))
      (Variables|Default|SetDialogueRef 0)
      (Variables|Default|SetDialogueIndex 0))))

(fn ConstructionScript)