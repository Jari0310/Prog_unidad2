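; BP_Chest is an interactable chest that the player can open only while holding a key.
; Interact casts the player pawn to BP_Player and sets IsOpen when HaveKey is true, without changing the key.
; A missing key or an already open chest prints a Spanish message instead.
; Each of these three outcomes adds an audio component; the graph grants no contents.
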(event EventInteract
  (if (Variables|Default|GetIsOpen)
    (Development|PrintString "Esta vacio")
    (AddComponent|AddAudioComponent false)
    (else
      (bind _asbp_player (Utilities|Casting|CastToBP_Player (Game|Player|GetPlayerPawn 0)))
      (if (Variables|/Game/01_Blueprints/01_player/BP_Player.BP_Player_C|GetHaveKey _asbp_player)
        (AddComponent|AddAudioComponent false)
        (Variables|Default|SetIsOpen true)
        (else
          (Development|PrintString "necesitas una llave")
          (AddComponent|AddAudioComponent false))))))

(fn ConstructionScript)